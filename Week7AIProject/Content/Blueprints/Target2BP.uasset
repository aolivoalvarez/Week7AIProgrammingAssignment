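; Target actor Blueprint that loses health when overlapped and awards the player a point when it dies.
; Any actor overlap decrements Health and prints the new value, with no check on what overlapped it.
; At zero or below, the target destroys itself, then casts player character 0 to PlayerBP and increments its Points.
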(event `self.ReceiveActorBeginOverlap`
  (params (OtherActor :type "Actor Object Reference"))
  ;[1 1 1] TargetHealth/Death
  (bind _result (`/Engine/EditorBlueprintResources/StandardMacros.DecrementInt` (`self.Health`))
    (:`  `
      (bind _output_get (set `self.Health` _result))
      (`KismetSystemLibrary.PrintString` (`KismetStringLibrary.Conv_IntToString` _output_get))
      (if (<= _output_get 0)
        (`self.K2_DestroyActor`)
        (bind _asplayer_bp (cast `/Game/Blueprints/PlayerBP` (`GameplayStatics.GetPlayerCharacter` 0)))
        (bind _result_2 (`/Engine/EditorBlueprintResources/StandardMacros.IncrementInt` (`/Game/Blueprints/PlayerBP.Points` _asplayer_bp))
          (:`  `
            (set `/Game/Blueprints/PlayerBP.Points` _result_2 _asplayer_bp)))))))

(fn `UserConstructionScript`)