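; Target1BP is an actor that moves in a loop between placed actors in its Places array.
; Each Tick it lerps from its current location toward the active place by DeltaSeconds times Speed, easing in as it nears, without sweeping.
; Once within the Distance threshold it increments Index, wrapping to zero past a hard-coded limit of 2 rather than the array's length.
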(event `self.ReceiveTick`
  (params (DeltaSeconds :type "Float (single-precision)"))
  (bind _index (`self.Index`))
  (bind _returnvalue (`self.K2_GetActorLocation` (`|GetArrayItem` (`self.Places`) _index)))
  ;[1 1 1] Lerp
  (`self.K2_SetActorLocation` (`KismetMathLibrary.VLerp` (`self.K2_GetActorLocation`) _returnvalue (* DeltaSeconds (`self.Speed`))))
  (if (<= (`KismetMathLibrary.Vector_Distance` (`self.K2_GetActorLocation`) _returnvalue) (`self.Distance`))
    (bind _result (`/Engine/EditorBlueprintResources/StandardMacros.IncrementInt` _index)
      (:`  `
        (if (> _result 2)
          (set `self.Index` 0))))))

(fn `UserConstructionScript`)